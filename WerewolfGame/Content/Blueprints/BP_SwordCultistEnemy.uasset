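; BP_SwordCultistEnemy is a sword-wielding cultist enemy that performs a melee attack through its EnemyAttack event.
; The attack swaps the Sword flipbook to a swing animation, plays a sound, and after a short delay spawns a BP_Attack actor at the AttackPosition component, owned and instigated by the enemy.
; It then restores the sword's default flipbook.
; BeginPlay, overlap and Tick add no logic.
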(event `self.ReceiveBeginPlay`)

(event `/Game/Blueprints/BPI_Enemy.EnemyAttack`
  (`PaperFlipbookComponent.SetFlipbook` (`self.Sword`) "/Game/Art/Cultist/Anim_SwordAttack.Anim_SwordAttack")
  (`GameplayStatics.PlaySound2D` "/Game/Audio/sword_sound.sword_sound" 1.0 1.0 0.0 null null)
  (`KismetSystemLibrary.Delay` 0.3)
  (`|SpawnActorFromClass` "/Game/Blueprints/BP_Attack.BP_Attack_C" (`SceneComponent.K2_GetComponentToWorld` (`self.AttackPosition`)) "Undefined" "OverrideRootScale" self self)
  (`PaperFlipbookComponent.SetFlipbook` (`self.Sword`) "/Game/Art/Cultist/Anim_Sword.Anim_Sword"))

(fn `UserConstructionScript`
  (`parent.UserConstructionScript`))