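; BP_Enemy is a side-scroller enemy that takes damage, awards score on death and hurts the player on contact.
; DoDamage lowers Health, optionally blocks attacks through BP_EnemyController, and flashes the flipbook red.
; A lethal hit adds ScoreValue via the game mode and destroys the actor, otherwise a timed Damaged flag briefly prevents further hits.
; Capsule hits damage SideScrollerCharacter and, if TakeDamage returns true, apply a frame-rate-scaled knockback force.
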(event `/Game/Blueprints/BPI_Enemy.DoDamage`
  (params (DamageAmount :type "Float (single-precision)"))
  ;[1 1 1] Defaut Enemy Damage function
  (if (not (`self.Damaged`))
    (bind _output_get (set `self.Health` (- (`self.Health`) DamageAmount)))
    (`KismetSystemLibrary.PrintString` (`KismetStringLibrary.Conv_DoubleToString` _output_get) true true (struct :`R` 1.0 :`G` 0.081415 :`B` 0.051568 :`A` 1.0))
    (if (`self.CanHitStun`)
      (bind _asbp_enemy_controller (cast `/Game/Blueprints/BP_EnemyController` (`self.GetController`)))
      (`/Game/Blueprints/BP_EnemyController.SetCanAttack` _asbp_enemy_controller false))
    (`PaperFlipbookComponent.SetSpriteColor` (`self.PaperFlipbook`) (struct :`R` 1.0 :`A` 1.0))
    (`KismetSystemLibrary.K2_SetTimerDelegate` (delegate `ResetMaterial`) 0.2)
    (if (<= (`self.Health`) 0.0)
      (bind _asside_scroller_game_mode (cast `/Game/Blueprints/SideScrollerGameMode` (`GameplayStatics.GetGameMode`)))
      (`/Game/Blueprints/SideScrollerGameMode.AddToScore` _asside_scroller_game_mode (`self.ScoreValue`))
      (`self.K2_DestroyActor`)
      (else
        (set `self.Damaged` true)
        (`KismetSystemLibrary.K2_SetTimerDelegate` (delegate `ResetDamaged`) 0.2)))))

(event `ResetDamaged`
  (set `self.Damaged` false))

(event `ResetMaterial`
  ;[1 1 1] Reset material
  (`PaperFlipbookComponent.SetSpriteColor` (`self.PaperFlipbook`) (struct :`R` 1.0 :`G` 1.0 :`B` 1.0 :`A` 1.0)))

(event `self.CapsuleComponent.OnComponentHit`
  (params (HitComponent :type "PrimitiveComponent Object Reference") (OtherActor :type "Actor Object Reference") (OtherComp :type "PrimitiveComponent Object Reference") (NormalImpulse :type "Vector Structure") (Hit :type "HitResult Structure (by ref)"))
  (bind _asside_scroller_character (cast `/Game/Blueprints/SideScrollerCharacter` OtherActor))
  (bind _tookdamage (`/Game/Blueprints/SideScrollerCharacter.TakeDamage` _asside_scroller_character 1.0))
  (if _tookdamage
    (bind _returnvalue_x (`KismetMathLibrary.BreakVector` (`self.GetActorRightVector` _asside_scroller_character)))
    (`CharacterMovementComponent.AddForce` (`Character.CharacterMovement` _asside_scroller_character) (* (`KismetMathLibrary.MakeVector` 0.0 _returnvalue_x) (* (/ (`GameplayStatics.GetWorldDeltaSeconds`) 0.016667) 15000000.0)))))

(fn `UserConstructionScript`)