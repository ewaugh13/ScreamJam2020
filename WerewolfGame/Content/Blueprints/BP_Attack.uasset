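; BP_Attack is a short-lived melee hitbox actor spawned by either the player or an enemy in a side-scroller.
; Its construction script takes the damage amount from the owning SideScrollerCharacter's attack stat, or from an enemy owner's AI Blackboard.
; Box overlaps ignore the owner, damage a BP_Enemy or SideScrollerCharacter, then destroy the actor, which otherwise removes itself after a brief delay.
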(event `self.ReceiveBeginPlay`
  (`KismetSystemLibrary.Delay` 0.1)
  (`self.K2_DestroyActor` :!label _label))

(event `self.Box.OnComponentBeginOverlap`
  (params (OverlappedComponent :type "PrimitiveComponent Object Reference") (OtherActor :type "Actor Object Reference") (OtherComp :type "PrimitiveComponent Object Reference") (OtherBodyIndex :type Integer) (bFromSweep :type Boolean) (SweepResult :type "HitResult Structure (by ref)"))
  (if (!= (`self.GetOwner`) OtherActor)
    (bind _asbp_enemy (cast `/Game/Blueprints/BP_Enemy` OtherActor)
      (:`then`
        (message `/Game/Blueprints/BPI_Enemy.DoDamage` _asbp_enemy (`self.DamageAmount`))
        (goto _label))
      (:`CastFailed`
        (bind _asside_scroller_character (cast `/Game/Blueprints/SideScrollerCharacter` OtherActor))
        (`/Game/Blueprints/SideScrollerCharacter.TakeDamage` _asside_scroller_character (`self.DamageAmount`))
        (goto _label)))))

(fn `UserConstructionScript`
  (bind _returnvalue (`self.GetOwner`))
  ;[1 1 1] Damage amount from player
  (bind _asside_scroller_character (cast `/Game/Blueprints/SideScrollerCharacter` _returnvalue)
    (:`then`
      (set `self.DamageAmount` (`/Game/Blueprints/SideScrollerCharacter.AttackDamageAmount` _asside_scroller_character)))
    (:`CastFailed`
      ;[1 1 1] Damage Amount from Enemy
      (bind _asbp_enemy (cast `/Game/Blueprints/BP_Enemy` _returnvalue))
      (bind _asbp_enemy_controller (cast `/Game/Blueprints/BP_EnemyController` (`AIBlueprintHelperLibrary.GetAIController` _asbp_enemy)))
      (set `self.DamageAmount` (`BlackboardComponent.GetValueAsFloat` (`AIController.Blackboard` _asbp_enemy_controller) "DamageAmount")))))