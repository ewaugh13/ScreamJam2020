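; BP_Arrow is a projectile actor that damages SideScrollerCharacters it hits.
; LaunchProjectile starts the initially inactive ProjectileMovement along Direction at Speed, with gravity disabled for straight flight.
; Capsule overlaps count only against components tagged KillCapsule on actors other than the owner, dealing DamageAmount to characters and destroying the arrow either way.
; Otherwise, the arrow destroys itself after a short lifetime delay started on BeginPlay.
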(event `self.ReceiveBeginPlay`
  (`KismetSystemLibrary.Delay` 5.0)
  (`self.K2_DestroyActor` :!label _label))

(event `self.Capsule.OnComponentBeginOverlap`
  (params (OverlappedComponent :type "PrimitiveComponent Object Reference") (OtherActor :type "Actor Object Reference") (OtherComp :type "PrimitiveComponent Object Reference") (OtherBodyIndex :type Integer) (bFromSweep :type Boolean) (SweepResult :type "HitResult Structure (by ref)"))
  (if (and (`ActorComponent.ComponentHasTag` OtherComp "KillCapsule") (!= (`self.GetOwner`) OtherActor))
    (bind _asside_scroller_character (cast `/Game/Blueprints/SideScrollerCharacter` OtherActor)
      (:`then`
        (`/Game/Blueprints/SideScrollerCharacter.TakeDamage` _asside_scroller_character (`self.DamageAmount`))
        (goto _label))
      (:`CastFailed`
        (goto _label)))))

(fn `LaunchProjectile`
  (`ProjectileMovementComponent.SetVelocityInLocalSpace` (`self.ProjectileMovement`) (* (`self.Direction`) (`self.Speed`)))
  (set `ProjectileMovementComponent.ProjectileGravityScale` 0.0 (`self.ProjectileMovement`))
  (`ActorComponent.Activate` (`self.ProjectileMovement`) true))

(fn `UserConstructionScript`
  (`ActorComponent.SetAutoActivate` (`self.ProjectileMovement`) false)
  (`SceneComponent.K2_SetWorldRotation` :`self` (`self.DefaultSceneRoot`)))